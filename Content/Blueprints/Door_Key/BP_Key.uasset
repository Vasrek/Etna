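; BP_Key is a colored key pickup that gives its Color to the player on overlap.
; When a BP_Player enters SphereCol, it calls AddKey, then hides the actor and disables its collision, restoring both after a short delay so the key respawns.
; The construction script sets the Sphere mesh material from the Color value.
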(event `self.SphereCol.OnComponentBeginOverlap`
  (params (OverlappedComponent :type "PrimitiveComponent Object Reference") (OtherActor :type "Actor Object Reference") (OtherComp :type "PrimitiveComponent Object Reference") (OtherBodyIndex :type Integer) (bFromSweep :type Boolean) (SweepResult :type "HitResult Structure (by ref)"))
  (bind _asbp_player (cast `/Game/Blueprints/BP_Player` OtherActor))
  (`/Game/Blueprints/BP_Player.AddKey` _asbp_player (`self.Color`))
  (`self.SetActorHiddenInGame` true)
  (`self.SetActorEnableCollision` false)
  (`KismetSystemLibrary.Delay` 4.0)
  (`self.SetActorHiddenInGame` false)
  (`self.SetActorEnableCollision` true))

(fn `UserConstructionScript`
  (switch `/Game/Blueprints/Door_Key/E_Color` (`self.Color`)
    (:`NewEnumerator6`
      (set `self.Material` "/Engine/BasicShapes/BasicShapeMaterial.BasicShapeMaterial"))
    (:`NewEnumerator0`
      (set `self.Material` "/AnimationSharing/AnimSharingBlue.AnimSharingBlue"))
    (:`NewEnumerator1`
      (set `self.Material` "/Engine/EngineMaterials/CubeMaterial.CubeMaterial"))
    (:`NewEnumerator2`
      (set `self.Material` "/AnimationSharing/AnimSharingGreen.AnimSharingGreen"))
    (:`NewEnumerator3`
      (set `self.Material` "/AnimationSharing/AnimSharingRed.AnimSharingRed")))
  (`PrimitiveComponent.SetMaterial` (`self.Sphere`) 0 (`self.Material`)))