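; BP_Door is a color-keyed door that sinks into the floor when a player holding the matching key overlaps its trigger box.
; The construction script sets the cube's material from the Color variable.
; A match starts a looping timer on OpenDoor, which interpolates the cube 500 units down and clears itself near the target.
; A mismatch shows a HUD message naming the required key, hidden on overlap end.
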(event `self.ReceiveBeginPlay`
  (bind _output_get (set `self.DefaultLoc` (`SceneComponent.K2_GetComponentLocation` (`self.Cube`))))
  (set `self.TargetLoc` (`KismetMathLibrary.MakeVector` (.x _output_get) (.y _output_get) (- (.z _output_get) 500.0))))

(event `self.Box.OnComponentBeginOverlap`
  (params (OverlappedComponent :type "PrimitiveComponent Object Reference") (OtherActor :type "Actor Object Reference") (OtherComp :type "PrimitiveComponent Object Reference") (OtherBodyIndex :type Integer) (bFromSweep :type Boolean) (SweepResult :type "HitResult Structure (by ref)"))
  (if (not (`self.IsDoorOpen?`))
    (bind _asbp_player (cast `/Game/Blueprints/BP_Player` OtherActor))
    (if (`|EnumEquality` (`/Game/Blueprints/BP_Player.CurrentKeyColor` _asbp_player) (`self.Color`))
      (`KismetSystemLibrary.K2_SetTimer` null "OpenDoor" 0.01 true)
      (set `self.IsDoorOpen?` true)
      (else
        (`/Game/Blueprints/UI/WBP_HUD.DisplayMessagePanel` (`/Game/Blueprints/BP_Player.HudRef` _asbp_player))
        (set `/Game/Blueprints/BP_Player.MessageToDisplay` (`|FormatText` "You must find the {color} key " (select `/Game/Blueprints/Door_Key/E_Color` (`self.Color`) :`NewEnumerator0` "Blue" :`NewEnumerator1` "Yellow" :`NewEnumerator2` "Green" :`NewEnumerator3` "Red" :!type "Text")) _asbp_player)))))

(event `self.Box.OnComponentEndOverlap`
  (params (OverlappedComponent :type "PrimitiveComponent Object Reference") (OtherActor :type "Actor Object Reference") (OtherComp :type "PrimitiveComponent Object Reference") (OtherBodyIndex :type Integer))
  (bind _asbp_player (cast `/Game/Blueprints/BP_Player` OtherActor))
  (`/Game/Blueprints/UI/WBP_HUD.HideMessagePanel` (`/Game/Blueprints/BP_Player.HudRef` _asbp_player)))

(fn `OpenDoor`
  (bind _cube (`self.Cube`))
  (bind _returnvalue (`KismetMathLibrary.VInterpTo` (`SceneComponent.K2_GetComponentLocation` _cube) (`self.TargetLoc`) (`GameplayStatics.GetWorldDeltaSeconds`) (`self.Speed`)))
  (`SceneComponent.K2_SetWorldLocation` _cube _returnvalue false false)
  (if (== _returnvalue (`self.TargetLoc`) :`ErrorTolerance` 5.0)
    (`KismetSystemLibrary.K2_ClearTimer` null "OpenDoor")))

(fn `UserConstructionScript`
  (switch `/Game/Blueprints/Door_Key/E_Color` (`self.Color`)
    (:`NewEnumerator6`
      (set `self.Material` "/Engine/BasicShapes/BasicShapeMaterial.BasicShapeMaterial"))
    (:`NewEnumerator0`
      (set `self.Material` "/AnimationSharing/AnimSharingBlue.AnimSharingBlue"))
    (:`NewEnumerator1`
      (set `self.Material` "/Engine/EngineMaterials/CubeMaterial.CubeMaterial"))
    (:`NewEnumerator2`
      (set `self.Material` "/AnimationSharing/AnimSharingGreen.AnimSharingGreen"))
    (:`NewEnumerator3`
      (set `self.Material` "/AnimationSharing/AnimSharingRed.AnimSharingRed")))
  (`PrimitiveComponent.SetMaterial` (`self.Cube`) 0 (`self.Material`)))