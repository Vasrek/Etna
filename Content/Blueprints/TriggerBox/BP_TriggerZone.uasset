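; BP_TriggerZone is a trigger box that acts as a death zone, checkpoint or level finish when BP_Player overlaps it.
; The TriggerZone variable selects the behavior: Death calls the player's Death, and Checkpoint sets the respawn transform from an Arrow component with unit scale.
; Win saves through GI_MyGameInstance, then opens the MainMenu level after a short delay.
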(event `self.Box.OnComponentBeginOverlap`
  (params (OverlappedComponent :type "PrimitiveComponent Object Reference") (OtherActor :type "Actor Object Reference") (OtherComp :type "PrimitiveComponent Object Reference") (OtherBodyIndex :type Integer) (bFromSweep :type Boolean) (SweepResult :type "HitResult Structure (by ref)"))
  (bind (_returnvalue_location _returnvalue_rotation) (`KismetMathLibrary.BreakTransform` (`SceneComponent.K2_GetComponentToWorld` (`self.Arrow`))))
  (bind _asbp_player (cast `/Game/Blueprints/BP_Player` OtherActor))
  (switch `/Game/Blueprints/TriggerBox/E_TriggerZone` (`self.TriggerZone`)
    (:`NewEnumerator0`
      (`/Game/Blueprints/BP_Player.Death` _asbp_player))
    (:`NewEnumerator1`
      (`/Game/Blueprints/BP_Player.SetNewRespawnTransform` _asbp_player (`KismetMathLibrary.MakeTransform` _returnvalue_location _returnvalue_rotation)))
    (:`NewEnumerator2`
      (bind _asgi_my_game_instance (cast `/Game/Blueprints/GI_MyGameInstance` (`GameplayStatics.GetGameInstance`)))
      (`/Game/Blueprints/GI_MyGameInstance.Save` _asgi_my_game_instance)
      (`KismetSystemLibrary.Delay` 0.2)
      (`GameplayStatics.OpenLevel` "MainMenu"))))

(fn `UserConstructionScript`)