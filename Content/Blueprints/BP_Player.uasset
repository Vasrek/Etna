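; BP_Player is the player character Blueprint, handling movement, camera look, respawning and a held key color.
; Axis inputs move it along control-yaw forward and right vectors, mouse axes drive pitch and yaw, and Jump starts and stops jumping.
; BeginPlay saves the spawn transform and adds WBP_HUD to the viewport.
; Death teleports the player to the saved transform, which SetNewRespawnTransform can replace, while AddKey sets CurrentKeyColor.
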(event `InputAxis|Forward/Backward`
  (params (AxisValue :type "Float (single-precision)"))
  (bind (_returnvalue_roll _returnvalue_pitch _returnvalue_yaw) (`KismetMathLibrary.BreakRotator` (`self.GetControlRotation`)))
  ;[1 0.6012 0] Base movement
  ;;[1 1 1] Input forward/backward/right/left
  (`self.AddMovementInput` (`KismetMathLibrary.GetForwardVector` (`KismetMathLibrary.MakeRotator` 0.0 0.0 _returnvalue_yaw)) AxisValue))

(event `InputAction|Jump`
  (params (Key :type "Key Structure"))
  ;[1 0.6012 0] Base movement
  ;;[1 1 1] Input action: Jump
  (:`Pressed`
    (`self.Jump`))
  (:`Released`
    (`self.StopJumping`)))

(event `InputAxis|Right/Left`
  (params (AxisValue :type "Float (single-precision)"))
  (bind (_returnvalue_roll _returnvalue_pitch _returnvalue_yaw) (`KismetMathLibrary.BreakRotator` (`self.GetControlRotation`)))
  ;[1 0.6012 0] Base movement
  ;;[1 1 1] Input forward/backward/right/left
  (`self.AddMovementInput` (`KismetMathLibrary.GetRightVector` (`KismetMathLibrary.MakeRotator` 0.0 0.0 _returnvalue_yaw)) AxisValue))

(event `InputAxis|MouseVertical`
  (params (AxisValue :type "Float (single-precision)"))
  ;[1 0.6012 0] Base movement
  ;;[1 1 1] Mouse input vertical/horizontal
  (`self.AddControllerPitchInput` AxisValue))

(event `InputAxis|MouseHorizontal`
  (params (AxisValue :type "Float (single-precision)"))
  ;[1 0.6012 0] Base movement
  ;;[1 1 1] Mouse input vertical/horizontal
  (`self.AddControllerYawInput` AxisValue))

(event `self.ReceiveBeginPlay`
  (set `self.RespawnTransform` (`self.GetTransform`))
  (bind _returnvalue (`|CreateWidget` "/Game/Blueprints/UI/WBP_HUD.WBP_HUD_C"))
  (bind _output_get (set `self.HudRef` _returnvalue))
  (`UserWidget.AddToViewport` _output_get 0))

(event `Death`
  (`self.K2_SetActorTransform` (`self.RespawnTransform`) false true))

(event `SetNewRespawnTransform`
  (params (NewRespawnTransform :type "Transform Structure"))
  (set `self.RespawnTransform` NewRespawnTransform))

(event `AddKey`
  (params (CurrentKeyColor :type "/Game/Blueprints/Door_Key/E_Color Enum" :default "NewEnumerator0"))
  (set `self.CurrentKeyColor` CurrentKeyColor))

(fn `UserConstructionScript`)