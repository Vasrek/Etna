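; Game instance that persists the player's best-run stats through an SG_PlayerStat save object.
; Load reads the save slot, or creates a new save object if none exists, caches the reference and writes it back to the slot.
; Save copies death count, score and HUD timer from BP_Player and writes to disk only when the current score beats the saved one.
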(event `Save`
  (bind _sg_statref (`self.SG_StatRef`))
  (bind _asbp_player (cast `/Game/Blueprints/BP_Player` (`GameplayStatics.GetPlayerCharacter` 0)))
  (if (not (<= (`/Game/Blueprints/BP_Player.TotalScore` _asbp_player) (`/Game/Blueprints/SG_PlayerStat.TotalScore` (`self.SG_StatRef`))))
    (set `/Game/Blueprints/SG_PlayerStat.TotalDeath` (`/Game/Blueprints/BP_Player.TotalDeathValue` _asbp_player) _sg_statref)
    (set `/Game/Blueprints/SG_PlayerStat.TotalScore` (`/Game/Blueprints/BP_Player.TotalScore` _asbp_player) _sg_statref)
    (set `/Game/Blueprints/SG_PlayerStat.TimerInSeconds` (`/Game/Blueprints/UI/WBP_HUD.Timer` (`/Game/Blueprints/BP_Player.HudRef` _asbp_player)) _sg_statref)
    (`GameplayStatics.SaveGameToSlot` (`self.SG_StatRef`) (`self.SaveGameString`))))

(event `Load`
  (bind _returnvalue (`GameplayStatics.DoesSaveGameExist` (`self.SaveGameString`)))
  (if _returnvalue
    (bind _returnvalue_2 (`GameplayStatics.LoadGameFromSlot` (`self.SaveGameString`)))
    (bind _assg_player_stat (cast `/Game/Blueprints/SG_PlayerStat` _returnvalue_2))
    (set `self.SG_StatRef` _assg_player_stat)
    (else
      (bind _returnvalue_3 (`GameplayStatics.CreateSaveGameObject` "/Game/Blueprints/SG_PlayerStat.SG_PlayerStat_C"))
      (set `self.SG_StatRef` _returnvalue_3)))
  (`GameplayStatics.SaveGameToSlot` (`self.SG_StatRef`) (`self.SaveGameString`)))